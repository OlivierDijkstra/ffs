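; BP_InteractionArea is an interaction zone actor that relays focus changes to its parent actor.
; ToggleFocus stores the focus state, notifies the parent through an interface message, and fetches the parent's interaction widget component the same way.
; It shows the widget only while focused and writes its Text variable into the WB_Interaction label, printing an error if the cast fails.
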(event Custom|ToggleFocus
  (params (Focused :type Boolean))
  (bind _output_get (Variables|Default|SetFocused Focused))
  (Class|BIInteraction|InterfaceToggleFocus(Message) (Actor|GetParentActor) _output_get)
  (bind _ref (Class|BIInteraction|GetInteractionWidgetRef(Message) (Actor|GetParentActor)))
  (Development|SetHiddeninGame _ref (not (Variables|Default|GetFocused)) false)
  (bind _aswb_interaction (Utilities|Casting|CastToWB_Interaction (UserInterface|GetWidget _ref))
    (:then
      (Rendering|Components|TextRender|SetText (Variables|/Game/Interaction/WB_Interaction.WB_Interaction_C|GetInteractableText _aswb_interaction) (Variables|Default|GetText)))
    (:CastFailed
      (Development|PrintString "FAILED TO CAST IN BP_INTERACTIONAREA"))))

(fn ConstructionScript)