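; Interaction component that lets the player focus on BP_InteractionArea actors and trigger instant or hold-to-interact actions.
; Each tick, a camera-forward line trace updates the focused area, toggling its highlight state and cancelling progress on focus loss.
; TryToInteract either fires immediately or runs a looping timer that fills the parent actor's WB_Interaction progress, resetting on release.
; Completed interactions call InteractOnServer, which sends an interface message to the area's parent actor.
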(event Custom|TryToInteract
  (params (In :type Boolean))
  (if In
    (if (Variables|Default|GetIsTractingInteractionArea)
      (bind _output_get (Variables|Default|SetInteraction%20Duration (Variables|/Game/Interaction/BP_InteractionArea.BP_InteractionArea_C|GetInteractionDuration (Variables|Default|GetFocusedInteractionArea))))
      (if (> _output_get 0.0)
        (bind _aswb_interaction (Utilities|GetWidget))
        (Variables|Default|SetCurrentInteractionWidgetRef _aswb_interaction)
        (bind _returnvalue (Utilities|Time|SetTimerbyEvent (delegate Custom|UpdateInteractionProgress) (Variables|Default|GetUpdateInteractionInterval) true))
        (Variables|Default|SetInteractionTimer _returnvalue)
        (else
          (CallFunction|InteractonServer (Variables|Default|GetFocusedInteractionArea)))))
    (else
      (CallFunction|StopInteraction))))

(event Custom|InteractOnServer
  (params (InteractionArea :type BP%20Interaction%20Area%20Object%20Reference))
  (Class|BIInteraction|InterfaceInteract(Message) (Actor|GetParentActor InteractionArea)))

(event Custom|UpdateInteractionProgress
  (bind _output_get (Variables|Default|SetInteractionProgress (+ (Variables|Default|GetInteractionProgress) (* (/ 1.0 (Variables|Default|GetInteraction%20Duration)) (Variables|Default|GetUpdateInteractionInterval)))))
  (Default|SetPercentage (Variables|Default|GetCurrentInteractionWidgetRef) _output_get)
  (if (>= (Variables|Default|GetInteractionProgress) 1.0)
    (CallFunction|StopInteraction)
    (CallFunction|InteractonServer (Variables|Default|GetFocusedInteractionArea))
    (CallFunction|StopInteraction)))

(event EventTick
  (params (DeltaSeconds :type Float%20%28single-precision%29))
  (CallFunction|Trace))

(fn Trace
  (bind _returnvalue (Game|GetPlayerCameraManager 0))
  (bind _returnvalue_2 (Transformation|GetActorLocation _returnvalue))
  (bind (_outhit _returnvalue_3) (Collision|LineTraceByChannel _returnvalue_2 (+ _returnvalue_2 (* (Math|Vector|GetForwardVector (Transformation|GetActorRotation _returnvalue)) (Variables|Default|GetTraceLength))) "TraceTypeQuery1" false 0 "None"))
  (if _returnvalue_3
    (if (!= (Variables|Default|GetFocusedActor) (.HitActor (Collision|BreakHitResult _outhit)))
      (Variables|Default|SetFocusedActor (.HitActor (Collision|BreakHitResult _outhit)))
      (CallFunction|TraceInteractionArea (== (Utilities|GetClass (.HitActor (Collision|BreakHitResult _outhit))) "/Game/Interaction/BP_InteractionArea.BP_InteractionArea_C")))
    (else
      (CallFunction|TraceInteractionArea false))))

(fn TraceInteractionArea
  (params (Trace :type Boolean))
  (if Trace
    (if (Variables|Default|GetIsTractingInteractionArea)
      (Default|ToggleFocus (Variables|Default|GetFocusedInteractionArea) false))
    (bind _asbp_interaction_area (Utilities|Casting|CastToBP_InteractionArea (Variables|Default|GetFocusedActor)))
    (bind _output_get (Variables|Default|SetFocusedInteractionArea _asbp_interaction_area))
    (Default|ToggleFocus _output_get true)
    (Variables|Default|SetIsTractingInteractionArea true)
    (elif (Variables|Default|GetIsTractingInteractionArea)
      (Variables|Default|SetIsTractingInteractionArea false)
      (Default|ToggleFocus (Variables|Default|GetFocusedInteractionArea) false)
      (Variables|Default|SetFocusedActor 0)
      (Variables|Default|SetFocusedInteractionArea 0)
      (CallFunction|StopInteraction))))

(fn StopInteraction
  (if (> (Variables|Default|GetInteractionProgress) 0.0)
    (Utilities|Time|ClearandInvalidateTimerbyHandle (Variables|Default|GetInteractionTimer))
    (Default|SetPercentage (Variables|Default|GetCurrentInteractionWidgetRef) 0.0)
    (Variables|Default|SetInteractionProgress 0.0)
    (Variables|Default|SetCurrentInteractionWidgetRef 0)))